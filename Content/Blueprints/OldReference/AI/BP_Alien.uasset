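; BP_Alien is an enemy AI pawn that chases the player, attacks in melee range and can be killed.
; A repeating AIMoveTo loop handles pursuit, while Tick halts movement to play a montage in range and reactivates it on completion.
; DamagePlayer applies hit damage but is not called within this Blueprint.
; At zero health it disables movement and collision, updates BP_Marine kills, notifies BP_MarsMarineGameMode, then destroys itself after a delay.
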(event EventTick
  (params (DeltaSeconds :type Float%20%28single-precision%29))
  ;[0.2125 1 0.3106] Move If Alive and Not Attacking
  (if (CallFunction|CanAttack)
    (CallFunction|DeactivateAIMovement)
    (Animation|Montage|PlayMontage (Variables|Character|GetMesh) 0
      (:OnCompleted
        (Components|Activation|Activate (Variables|Character|GetCharacterMovement) false)))))

(event Game|Damage|EventAnyDamage
  (params (Damage :type Float%20%28single-precision%29) (DamageType :type Damage%20Type%20Object%20Reference) (InstigatedBy :type Controller%20Object%20Reference) (DamageCauser :type Actor%20Object%20Reference))
  ;[1 0.04167 0.04167] Take Damage
  (if (CallFunction|IsAlive)
    (bind _newhealth (CallFunction|DecreaseHealth Damage))
    (if (== _newhealth 0.0)
      (CallFunction|KillAI)
      (Utilities|FlowControl|Delay 3.0)
      (Actor|DestroyActor))))

(event EventBeginPlay
  ;[0.1729 0.2596 1] Follow Player
  (Variables|Default|SetHealth (Variables|Default|GetMaxHealth))
  (if (CallFunction|IsAlive) :!label _label
    (AI|AIMoveTo self "0, 0, 0" (Game|GetPlayerCharacter 0) (- (Variables|Default|GetAttackRange) 4e+01) false
      (:OnSuccess
        _)
      (:OnFail
        _))
    (Utilities|FlowControl|Delay 0.2)
    (goto _label)))

(fn ConstructionScript)

(fn IsinAtkRange
  (return (<= (Transformation|GetDistanceTo (Game|GetPlayerCharacter 0)) (Variables|Default|GetAttackRange))))

(fn IsAttacking
  (return (Animation|Montage|MontageIsPlaying (Components|SkeletalMesh|GetAnimInstance (Variables|Character|GetMesh)) 0)))

(fn DamagePlayer
  (if (CallFunction|IsAlive)
    (Game|Damage|ApplyDamage (Game|GetPlayerCharacter 0) (Variables|Default|GetDamagePerHit) 0 0)))

(fn DecreaseHealth
  (params (Damage :type Float%20%28single-precision%29))
  (bind _output_get (Variables|Default|SetHealth (Math|Float|Clamp(Float) (- (Variables|Default|GetHealth) Damage) 0.0 (Variables|Default|GetMaxHealth))))
  (return _output_get))

(fn KillAI
  (Variables|Default|SetIsDead true)
  (CallFunction|DeactivateAIMovement)
  (Collision|SetActorEnableCollision false)
  (bind _asbp_marine (Utilities|Casting|CastToBP_Marine (Game|GetPlayerCharacter 0)))
  (Default|IncreaseKills _asbp_marine)
  (bind _asbp_mars_marine_game_mode (Utilities|Casting|CastToBP_MarsMarineGameMode (Game|GetGameMode)))
  (Default|AlienDeath _asbp_mars_marine_game_mode self))

(fn DeactivateAIMovement
  (bind _charactermovement (Variables|Character|GetCharacterMovement))
  (Components|Movement|StopMovementImmediately _charactermovement)
  (Components|Activation|Deactivate _charactermovement))

(fn IsAlive
  (return (not (Variables|Default|GetIsDead))))

(fn CanAttack
  (return (Math|Boolean|ANDBoolean (CallFunction|IsinAtkRange) (not (CallFunction|IsAttacking)) (CallFunction|IsAlive))))