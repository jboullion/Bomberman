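; Bomberman-style bomb actor that detonates in a cross along the block grid after its fuse animation.
; A timeline drives material glow and body scale, then calls Explode, which decrements the owning player's bomb count and copies their blast radius.
; Explosion paths step block by block in four directions, spawning Niagara effects and radial damage.
; Line traces stop each path at static walls or the first destructible, which takes point damage.
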(event EventBeginPlay
  (Variables|Default|SetStartScale (.scale (Transformation|GetRelativeTransform (Variables|Default|GetBombBody))))
  (bind _glow (Timeline|AnimateBomb Play)
    (:Update
      (Rendering|Material|SetScalarParameterValue (Variables|Default|GetMaterial) "Glow" _glow :!class /Script/Engine.MaterialInstanceDynamic)
      (Transformation|SetWorldScale3D (Variables|Default|GetBombBody) (* (Variables|Default|GetStartScale) (+ _glow 1.0))))
    (:Finished
      (CallFunction|Explode))))

(fn ConstructionScript
  (bind _bombbody (Variables|Default|GetBombBody))
  (bind _returnvalue (Rendering|Material|GetMaterials _bombbody))
  (bind _returnvalue_2 (Rendering|Material|CreateDynamicMaterialInstance (Utilities|Array|Get(acopy) _returnvalue (Utilities|Array|FindItem _returnvalue "/Game/Meshes/Bomb/Bomb001.Bomb001")) "Bomb001" :!class /Script/Engine.KismetMaterialLibrary))
  (bind _output_get (Variables|Default|SetMaterial _returnvalue_2))
  (Rendering|Material|SetMaterial (Variables|Default|GetBombBody) 0 _output_get))

(fn Explode
  (CallFunction|SetupBomb)
  (Audio|PlaySound2D "/Game/Music/Explosions.Explosions" 1.0 1.0 0.0 0 0)
  (Class|PlayerCameraManager|PlayCameraShake (Game|GetPlayerCameraManager 0) "/Game/Blueprints/BP_CameraShake.BP_CameraShake_C" 1.0 "World" "0, 0, 0")
  ;[1 1 1] Directional Explosions
  (CallFunction|GetExplosionPaths)
  (Actor|DestroyActor))

(fn GetExplosionPaths
  ;[1 1 1] CenterExplosion
  (CallFunction|ApplyDamageandSpawnParticle (Transformation|GetActorLocation))
  (Utilities|FlowControl|Sequence
    (:then_0
      ;[1 1 1] Vertical Paths
      (CallFunction|MakeExplosionPath "1.000000, 0, 0"))
    (:then_1
      (CallFunction|MakeExplosionPath "-1.000000, 0, 0"))
    (:then_2
      ;[1 1 1] Horizontal Path
      (CallFunction|MakeExplosionPath "0.000000,1.000000, 0"))
    (:then_3
      (CallFunction|MakeExplosionPath "0.000000,-1.000000, 0"))))

(fn SpawnImpactHit
  (params (Hit%20Location :type Vector))
  (Effects|SpawnEmitteratLocation "/Game/Particles/Explosion.Explosion" Hit%20Location))

(fn GetBombRange
  (return (* (Variables|Default|GetDamageRadius) (Variables|Default|GetBlockSize))))

(fn Countdown
  (Utilities|Time|SetTimerbyFunctionName 0 "Explode" (Variables|Default|GetLifetimeSeconds)))

(fn ExplosionCheckPath
  (params (Start :type Vector) (End :type Vector))
  (bind _outhits (Class|KismetSystemLibrary|LineTraceMultiforObjects Start End (Utilities|Array|MakeArray "ObjectTypeQuery6" "ObjectTypeQuery1") false 0 "ForDuration" true))
  (if (> (Utilities|Array|Length _outhits) 0)
    (bind _array_element (Utilities|Array|ForEachLoopwithBreak _outhits :!label _label)
      (:LoopBody
        (if (Utilities|Enum|Equal(Enum) (Utilities|String|EnumtoString (Collision|GetCollisionResponsetoChannel (.HitComponent (Collision|BreakHitResult _array_element)) "ECC_WorldStatic")) "Block")
          (goto _label Break)
          (else
            (Game|Damage|ApplyPointDamage (.HitActor (Collision|BreakHitResult _array_element)) (Variables|Default|GetDamage) (.ImpactPoint (Collision|BreakHitResult _array_element)) _array_element)))))))

(fn ApplyDamageandSpawnParticle
  (params (ExplosionPoint :type Vector))
  (Niagara|SpawnSystematLocation "/Game/Particles/Systems/NS_Explosion.NS_Explosion" ExplosionPoint "0, 0, 0" "0.250000,0.250000,0.250000")
  (Game|Damage|ApplyRadialDamage (Variables|Default|GetDamage) ExplosionPoint (/ (Variables|Default|GetBlockSize) 2.0) 0 0 self 0 true "ECC_WorldStatic"))

(fn MakeExplosionPath
  (params (PathVector :type Vector))
  ;[1 1 1] Step Along Each Block on the Path
  (bind _index (Utilities|FlowControl|ForLoopwithBreak 1 (Variables|Default|GetDamageRadius) :!label _label)
    (:LoopBody
      (if (CallFunction|DetectNonDestructible (+ (* PathVector (* _index (Variables|Default|GetBlockSize))) (Transformation|GetActorLocation)))
        (goto _label Break)
        (elif (CallFunction|DetectDestructible (+ (* PathVector (* _index (Variables|Default|GetBlockSize))) (Transformation|GetActorLocation)))
          (goto _label Break)
          (else
            ;[1 1 1] We Hit No Blocks so place explosion here
            (CallFunction|ApplyDamageandSpawnParticle (+ (* PathVector (* _index (Variables|Default|GetBlockSize))) (Transformation|GetActorLocation)))))))))

(fn DetectNonDestructible
  (params (End :type Vector))
  (bind _outhit (Collision|LineTraceForObjects (Transformation|GetActorLocation) End (Utilities|Array|MakeArray "ObjectTypeQuery1") false 0 "None"))
  (return (.bBlockingHit (Collision|BreakHitResult _outhit))))

(fn DetectBlockingHit
  (params (Location :type Vector))
  (bind _outhit (Collision|LineTraceForObjects (Transformation|GetActorLocation) "0, 0, 0" (Utilities|Array|MakeArray "ObjectTypeQuery6" "ObjectTypeQuery3") false 0 "None")))

(fn DetectDestructible
  (params (End :type Vector))
  ;[1 1 1] If we detect a destructible block, do point damage. This gives us the best explosion effect
  (bind _outhit (Collision|LineTraceForObjects (Transformation|GetActorLocation) End (Utilities|Array|MakeArray "ObjectTypeQuery6") false 0 "None"))
  (if (.bBlockingHit (Collision|BreakHitResult _outhit))
    (Game|Damage|ApplyPointDamage (.HitActor (Collision|BreakHitResult _outhit)) (Variables|Default|GetDamage) (.ImpactPoint (Collision|BreakHitResult _outhit)) _outhit 0 self)
    (Niagara|SpawnSystematLocation "/Game/Particles/Systems/NS_Explosion.NS_Explosion" End "0, 0, 0" "0.250000,0.250000,0.250000")
    (return (.bBlockingHit (Collision|BreakHitResult _outhit)))
    (else
      (return false))))

(fn DetectPlayer
  (params (End :type Vector))
  (bind _outhit (Collision|LineTraceForObjects (Transformation|GetActorLocation) End (Utilities|Array|MakeArray "ObjectTypeQuery3") false 0 "None"))
  (return (.bBlockingHit (Collision|BreakHitResult _outhit))))

(fn SetupBomb
  (bind _asbp_player (Utilities|Casting|CastToBP_Player (Components|GetOwner)))
  (Math|Integer|DecrementInt (Variables|/Game/Blueprints/Characters/BP_Player.BP_Player_C|GetCurrentBombs _asbp_player)
    (:%20%20
      (Variables|Default|SetDamageRadius (Variables|/Game/Blueprints/Characters/BP_Player.BP_Player_C|GetBombRadius _asbp_player))
      (return))))

(fn AnimateCountdown
  (Rendering|Material|SetScalarParameterValue (Variables|Default|GetMaterial) "Frequency" (Variables|Default|GetLifetimeSeconds) :!class /Script/Engine.MaterialInstanceDynamic))