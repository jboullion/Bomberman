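; Bomberman-style timed bomb actor that explodes after its lifetime, plays a sound and destroys itself.
; The blast traces four axis-aligned paths from the bomb, with range set by DamageRadius times BlockSize.
; Each multi-object trace applies point damage to blocking hits until it meets a component that blocks WorldStatic, which stops that path.
; An unconnected radial impulse explosion and an uncalled impact-emitter helper remain in the asset.
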(event EventBeginPlay
  (Utilities|Time|SetTimerbyFunctionName 0 "Explode" (Variables|Default|GetLifetimeSeconds)))

(fn ConstructionScript)

(fn Explode
  (Audio|PlaySound2D "/Game/Music/Explosions.Explosions" 1.0 1.0 0.0 0 0)
  ;[1 1 1] Directional Explosion
  (CallFunction|GetExplosionPaths)
  (Actor|DestroyActor))

(fn GetExplosionPaths
  (bind _bombrange (CallFunction|GetBombRange))
  (bind _bombrange_2 (CallFunction|GetBombRange))
  (bind _returnvalue (Math|Vector|MakeVector 0.0 1.0 0.0))
  (bind _returnvalue_2 (Math|Vector|MakeVector 1.0 0.0 0.0))
  (bind _returnvalue_3 (* _returnvalue_2 _bombrange))
  (bind _returnvalue_4 (* _returnvalue _bombrange_2))
  (Utilities|FlowControl|Sequence
    (:then_0
      ;[1 1 1] Vertical Paths
      (CallFunction|PathExplosion _returnvalue_3))
    (:then_1
      (CallFunction|PathExplosion (* _returnvalue_3 -1.0)))
    (:then_2
      ;[1 1 1] Horizontal Path
      (CallFunction|PathExplosion _returnvalue_4))
    (:then_3
      (CallFunction|PathExplosion (* _returnvalue_4 -1.0)))))

(fn PathExplosion
  (params (Path :type Vector))
  (bind _self self)
  (bind _returnvalue (Transformation|GetActorLocation _self))
  (bind _outhits (Class|KismetSystemLibrary|LineTraceMultiforObjects _returnvalue (+ _returnvalue Path) (Utilities|Array|MakeArray "ObjectTypeQuery6" "ObjectTypeQuery1") false 0 "ForDuration" true))
  (if (> (Utilities|Array|Length _outhits) 0)
    (bind _array_element (Utilities|Array|ForEachLoopwithBreak _outhits :!label _label)
      (:LoopBody
        (if (Utilities|Enum|Equal(Enum) (Utilities|String|EnumtoString (Collision|GetCollisionResponsetoChannel (.HitComponent (Collision|BreakHitResult _array_element)) "ECC_WorldStatic")) "Block")
          (goto _label Break)
          (elif (.bBlockingHit (Collision|BreakHitResult _array_element))
            (Game|Damage|ApplyPointDamage (.HitActor (Collision|BreakHitResult _array_element)) (Variables|Default|GetDamage) (.ImpactPoint (Collision|BreakHitResult _array_element)) _array_element)))))))

(fn SpawnImpactHit
  (params (Hit%20Location :type Vector))
  (Effects|SpawnEmitteratLocation "/Game/Particles/Explosion.Explosion" Hit%20Location))

(fn GetBombRange
  (return (* (Variables|Default|GetDamageRadius) (Variables|Default|GetBlockSize))))

(fn Countdown
  (Utilities|Time|SetTimerbyFunctionName 0 "Explode" (Variables|Default|GetLifetimeSeconds)))