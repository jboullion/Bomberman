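; BP_Cannon is an automatic cannon actor that repeatedly fires BP_Projectile from the moment play begins.
; After a FireRate delay, it spawns a scaled projectile at the BallSpawn component's transform and plays the Recoil timeline.
; The timeline animates the barrel's relative Y location, and its Cannon Fired event track loops back to the delay for the next shot.
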(event EventBeginPlay
  (Utilities|FlowControl|Delay (Variables|CannonProperties|GetFireRate) :!label _label)
  (CallFunction|SpawnProjectile)
  (bind _cannon_barrel_location (Timeline|Recoil PlayFromStart)
    (:Update
      (CallFunction|MoveCannonBarrel _cannon_barrel_location))
    (:Cannon%20Fired
      (goto _label))))

(fn ConstructionScript)

(fn SpawnProjectile
  (bind _ballspawn (Variables|Default|GetBallSpawn))
  (Game|SpawnActorfromClass "/Game/Blueprints/OldReference/Actors/Projectiles/BP_Projectile.BP_Projectile_C" (Math|Transform|MakeTransform (Transformation|GetWorldLocation _ballspawn) (Transformation|GetWorldRotation _ballspawn) (Math|Conversions|ToVector(Float) (Variables|CannonProperties|GetProjectileScale))) "Undefined" 0 0))

(fn MoveCannonBarrel
  (params (BarrelLocation :type Float%20%28single-precision%29))
  (Transformation|SetRelativeLocation (Variables|Default|GetBarrel) (Math|Vector|MakeVector 0.0 BarrelLocation 0.0) false false))