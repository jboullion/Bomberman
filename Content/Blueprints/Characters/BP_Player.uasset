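; Player character Blueprint that moves on world axes, carries and drops bombs, tracks score, and creates the HUD.
; Movement input turns the control rotation toward velocity; thumbstick and smoothed mouse aiming functions exist but are never called here.
; Holding HoldBomb spawns and attaches a BP_Bomb at BombSocket; releasing detaches it, snaps it to a 100-unit grid and starts its countdown.
; Any key press updates the GamepadActive flag.
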(event Custom|AddScore
  ;[0 0.02836 1] State Tracking
  (Math|Integer|IncrementInt (Variables|Default|GetScore)))

(event EventBeginPlay
  ;[1 1 1] UI
  (bind _returnvalue (UserInterface|CreateWidget "/Game/UI/BP_Hud.BP_Hud_C"))
  (UserInterface|Viewport|AddtoViewport _returnvalue 0))

(event Input|ActionEvents|InputActionHoldBomb
  (params (Key :type Key%20Structure :default "None"))
  ;[1 0.071 0.04116] Bomb
  (:Pressed
    (CallFunction|HoldBomb))
  (:Released
    (CallFunction|DropBomb)))

(event Input|AxisEvents|InputAxisMoveRight
  (params (AxisValue :type Float%20%28single-precision%29))
  ;[0.1188 1 0.1619] Movement
  (Pawn|Input|AddMovementInput "0.000000,1.000000, 0" AxisValue false)
  (CallFunction|UpdateRotation))

(event Input|AxisEvents|InputAxisMoveUp
  (params (AxisValue :type Float%20%28single-precision%29))
  ;[0.1188 1 0.1619] Movement
  (Pawn|Input|AddMovementInput "1.000000,0.000000, 0" AxisValue false)
  (CallFunction|UpdateRotation))

(event Input|KeyboardEvents|AnyKey
  (params (Key :type Key%20Structure :default "None"))
  ;[0.1188 1 0.1619] Movement
  (:Pressed
    (Variables|Default|SetGamepadActive (Class|KismetInputLibrary|KeyIsGamepadKey Key))))

(fn ConstructionScript)

(fn UpdateRotation
  (bind _returnvalue (Game|GetPlayerCharacter 0))
  (bind _returnvalue_2 (Transformation|GetVelocity _returnvalue))
  (bind (_x _y) (Math|Vector|BreakVector _returnvalue_2))
  (if (or (> (Math|Float|Absolute(Float) _x) 0.0) (> (Math|Float|Absolute(Float) _y) 0.0))
    (Pawn|SetControlRotation (Game|GetPlayerController 0) (Math|Rotator|MakeRotfromX _returnvalue_2))))

(fn ThumbstickRotation
  (if (CallFunction|IsThumbstickAboveDeadzone)
    (Pawn|SetControlRotation (Game|GetPlayerController 0) (CallFunction|GetThumbstickAimDirection))))

(fn GetThumbstickAimDirection
  (return (Math|Rotator|MakeRotator 0.0 0.0 (Class|KismetMathLibrary|DegAtan2 (Input|AxisValues|GetThumbstickAimRight) (* (Input|AxisValues|GetThumbstickAimUp) -1.0)))))

(fn UpdateMouseRotation
  (if (CallFunction|IsMouseAboveDeadzone)
    (Pawn|SetControlRotation (Game|GetPlayerController 0) (CallFunction|GetMouseAimDirection))))

(fn GetMouseAimDirection
  (bind _returnvalue (CallFunction|GetMouseVelocity))
  (return (Math|Interpolation|RInterpTo (Pawn|GetControlRotation (Game|GetPlayerController 0) :!class /Script/Engine.Controller) (Math|Rotator|MakeRotator 0.0 0.0 (Class|KismetMathLibrary|DegAtan2 (.x _returnvalue) (.y _returnvalue))) (Utilities|Time|GetWorldDeltaSeconds) (Variables|Default|GetMouseSmoothing))))

(fn GetMouseVelocity
  (bind _returnvalue (Game|GetPlayerController 0))
  (bind (_deltax _deltay) (Class|PlayerController|GetInputMouseDelta _returnvalue))
  (return (/ (Math|Vector2D|MakeVector2D _deltax _deltay) (Utilities|Time|GetWorldDeltaSeconds))))

(fn IsMouseAboveDeadzone
  (return (> (Math|Vector2D|Vector2DLength (CallFunction|GetMouseVelocity)) (Variables|Default|GetMouseDeadzone))))

(fn IsThumbstickAboveDeadzone
  (return (> (Math|Vector2D|Vector2DLength (Math|Vector2D|MakeVector2D (Input|AxisValues|GetThumbstickAimUp) (Input|AxisValues|GetThumbstickAimRight))) (Variables|Default|GetThumbstickDeadzone))))

(fn UpdateKeyboardRotation
  (bind _returnvalue (Game|GetPlayerCharacter 0))
  (bind _returnvalue_2 (Transformation|GetVelocity _returnvalue))
  (bind (_x _y) (Math|Vector|BreakVector _returnvalue_2))
  (if (or (> (Math|Float|Absolute(Float) _x) 0.0) (> (Math|Float|Absolute(Float) _y) 0.0))
    (Pawn|SetControlRotation (Game|GetPlayerController 0) (Math|Rotator|MakeRotfromX _returnvalue_2))))

(fn HoldBomb
  (if (not (Variables|Default|GetHoldingBomb))
    (Variables|Default|SetHoldingBomb true)
    (bind _returnvalue (Game|SpawnActorfromClass "/Game/Blueprints/Actors/BP_Bomb.BP_Bomb_C" (Math|Transform|MakeTransform (Transformation|GetSocketLocation (Variables|Default|GetBombSocket) "None") "0, 0, 0" "1,1,1") "Undefined" 0 0))
    (bind _output_get (Variables|Default|SetCurrentBomb _returnvalue))
    (Transformation|AttachActorToActor _output_get self "None" "KeepWorld" "KeepRelative" "KeepRelative" true)))

(fn DropBomb
  (bind _currentbomb (Variables|Default|GetCurrentBomb))
  (bind _returnvalue (Transformation|GetActorLocation _currentbomb))
  (Variables|Default|SetHoldingBomb false)
  (Utilities|IsValid _currentbomb
    (:Is%20Valid
      (Transformation|DetachFromActor _currentbomb "KeepWorld" "KeepWorld" "KeepWorld")
      (Transformation|SetActorLocation _currentbomb (Math|Vector|MakeVector (* (Math|Float|Round (/ (.x _returnvalue) 1e+02)) 1e+02) (* (Math|Float|Round (/ (.y _returnvalue) 1e+02)) 1e+02) 5e+01) false false)
      (Default|Countdown _currentbomb))))