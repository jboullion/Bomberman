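; BP_GridManager is a grid manager actor that spawns an X by Y grid of BP_GridBase actors when play begins.
; Nested loops space the cells by Size on a flat plane, offset by half the grid extent to roughly center them on the manager's location.
; Each spawned cell is stored in BaseArray, and debug prints show a greeting and every spawn position.
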(event EventBeginPlay
  (bind _x (Variables|Default|GetX))
  (bind _y (Variables|Default|GetY))
  (bind _size (Variables|Default|GetSize))
  (bind _size_2 (Variables|Default|GetSize))
  (Development|PrintString "Hello")
  (for _index (range 1 _x)
    (for _index_2 (range 1 _y)
      (Development|PrintString (Utilities|String|Append "X" (Utilities|String|ToString(Float) (.X (Math|Vector|BreakVector (+ (Math|Vector|MakeVector (Math|Conversions|ToFloat(Integer) (- (* _index _size) (/ (* _x _size_2) 2))) (Math|Conversions|ToFloat(Integer) (- (* _index_2 _size) (/ (* _y _size_2) 2))) 0.0) (Transformation|GetActorLocation))))) ", Y" (Utilities|String|ToString(Float) (.Y (Math|Vector|BreakVector (+ (Math|Vector|MakeVector (Math|Conversions|ToFloat(Integer) (- (* _index _size) (/ (* _x _size_2) 2))) (Math|Conversions|ToFloat(Integer) (- (* _index_2 _size) (/ (* _y _size_2) 2))) 0.0) (Transformation|GetActorLocation))))) ", Z" (Utilities|String|ToString(Float) (.Z (Math|Vector|BreakVector (+ (Math|Vector|MakeVector (Math|Conversions|ToFloat(Integer) (- (* _index _size) (/ (* _x _size_2) 2))) (Math|Conversions|ToFloat(Integer) (- (* _index_2 _size) (/ (* _y _size_2) 2))) 0.0) (Transformation|GetActorLocation)))))))
      (bind _returnvalue (Game|SpawnActorfromClass "/Game/Blueprints/Grid/BP_GridBase.BP_GridBase_C" (Math|Transform|MakeTransform (+ (Math|Vector|MakeVector (Math|Conversions|ToFloat(Integer) (- (* _index _size) (/ (* _x _size_2) 2))) (Math|Conversions|ToFloat(Integer) (- (* _index_2 _size) (/ (* _y _size_2) 2))) 0.0) (Transformation|GetActorLocation))) "AlwaysSpawn" 0 0))
      (Utilities|Array|Add (Variables|Default|GetBaseArray) _returnvalue))))

(event Collision|EventActorBeginOverlap
  (params (OtherActor :type Actor%20Object%20Reference)))

(event EventTick
  (params (DeltaSeconds :type Float%20%28single-precision%29)))

(fn ConstructionScript)