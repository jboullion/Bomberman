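; BP_Crystal is a pickup crystal that flies to the player when overlapped, then destroys itself.
; On player overlap it caches its location, scale and light intensity, then plays the MoveTo timeline.
; Separate timeline tracks drive lerps toward the player pawn's live position, zero scale and zero light intensity.
; No reward or inventory logic is present, only the collection effect.
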(event Collision|EventActorBeginOverlap
  (params (OtherActor :type Actor%20Object%20Reference))
  (Utilities|IsPlayer OtherActor
    (:true
      (CallFunction|StoreStartingValues)
      (bind (_direction _movementprogress _scaleprogress _lightintensity) (Timeline|Move%20To Play)
        (:Update
          (CallFunction|MovetoPlayer _movementprogress)
          (CallFunction|ScaleCrystal _scaleprogress)
          (CallFunction|AdjustLight _lightintensity))
        (:Finished
          (Actor|DestroyActor))))))

(fn ConstructionScript)

(fn MovetoPlayer
  (params (Alpha :type Float%20%28single-precision%29))
  (Transformation|SetActorLocation (Math|Vector|Lerp(Vector) (Variables|Default|GetStart%20Location) (Transformation|GetActorLocation (Game|Player|GetPlayerPawn 0)) Alpha) false false))

(fn StoreStartingValues
  (Variables|Default|SetStart%20Location (Transformation|GetActorLocation))
  (Variables|Default|SetStartScale (Transformation|GetActorScale3D))
  (Variables|Default|SetStartLightIntensity (Variables|/Script/Engine.LightComponentBase|GetIntensity (Variables|Default|GetPointLight))))

(fn ScaleCrystal
  (params (Alpha :type Float%20%28single-precision%29))
  (Transformation|SetActorScale3D (Math|Vector|Lerp(Vector) (Variables|Default|GetStartScale) "0, 0, 0" Alpha)))

(fn AdjustLight
  (params (NewIntensity :type Float%20%28single-precision%29))
  (Rendering|Components|Light|SetIntensity (Variables|Default|GetPointLight) (Math|Float|Lerp (Variables|Default|GetStartLightIntensity) 0.0 NewIntensity)))