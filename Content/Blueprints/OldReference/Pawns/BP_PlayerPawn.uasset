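; BP_PlayerPawn is a player pawn that rolls its static mesh using torque from movement input and dies on any damage.
; Forward/backward and right/left axes add acceleration-change torque around Y and X, scaled by MoveSpeed.
; Any damage triggers a once-only camera fade with audio in TakeDamage, waits for FadeDuration, then restarts the level.
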(event EventBeginPlay)

(event Collision|EventActorBeginOverlap
  (params (OtherActor :type Actor%20Object%20Reference)))

(event EventTick
  (params (DeltaSeconds :type Float%20%28single-precision%29)))

(event Game|Damage|EventAnyDamage
  (params (Damage :type Float%20%28single-precision%29) (DamageType :type Damage%20Type%20Object%20Reference) (InstigatedBy :type Controller%20Object%20Reference) (DamageCauser :type Actor%20Object%20Reference))
  (CallFunction|TakeDamage)
  (Utilities|FlowControl|Delay (Variables|Default|GetFadeDuration))
  (Utilities|RestartLevel))

(event Input|AxisEvents|InputAxisForwardBackwards
  (params (AxisValue :type Float%20%28single-precision%29))
  ;[0.1994 1 0.1886] Movement
  (Class|PrimitiveComponent|AddTorqueinRadians (Variables|Default|GetStaticMesh) (Math|Vector|MakeVector 0.0 (* AxisValue (Variables|Default|GetMoveSpeed)) 0.0) "None" true))

(event Input|AxisEvents|InputAxisRightLeft
  (params (AxisValue :type Float%20%28single-precision%29))
  ;[0.1994 1 0.1886] Movement
  (Class|PrimitiveComponent|AddTorqueinRadians (Variables|Default|GetStaticMesh) (Math|Vector|MakeVector (* AxisValue (Variables|Default|GetMoveSpeed)) 0.0 0.0) "None" true))

(fn ConstructionScript)

(fn TakeDamage
  (Utilities|FlowControl|DoOnce false
    (:Completed
      (CameraFades|StartCameraFade :self (Game|GetPlayerCameraManager 0) :ToAlpha 1.0 :Duration (Variables|Default|GetFadeDuration) :bShouldFadeAudio true :bHoldWhenFinished true))))